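; BP_DreamMooaToonTools is a placeable control actor that exposes MooaToon toon-rendering settings and applies them from its construction script.
; SetCVars pushes color ramp, rim light and hair shadow values to r.Mooa console variables, issuing commands only where values differ.
; SetPP writes exposure, light, shadow, GI and rim light settings into a post process component.
; That component comes from PostActor by index; otherwise the actor enables and uses its own.
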(fn `GetPostComponent`
  (returns (ReturnValue :type "PostProcessComponent Object Reference"))
  (bind _postactor (`self.PostActor`))
  (bind _postcomponentindex (`self.PostComponentIndex`))
  (bind _postprocess (`self.PostProcess`))
  (bind _returnvalue (`self.K2_GetComponentsByClass` _postactor "/Script/Engine.PostProcessComponent"))
  (bind _returnvalue_2 (`KismetArrayLibrary.Array_IsValidIndex` _returnvalue _postcomponentindex))
  (set `PostProcessComponent.bEnabled` (not _returnvalue_2) (`self.PostProcess`))
  (return (select `bool` (`KismetSystemLibrary.IsValid` _postactor) :`false` _postprocess :`true` (select `bool` _returnvalue_2 :`false` _postprocess :`true` (`|GetArrayItem` _returnvalue _postcomponentindex)))))

(fn `SetCVar`
  (params (`Var Name` :type String) (Value :type "Float (double-precision)"))
  (bind _returnvalue (`KismetSystemLibrary.GetConsoleVariableFloatValue` `Var Name`))
  (if (!= _returnvalue Value)
    (`KismetSystemLibrary.ExecuteConsoleCommand` (`KismetStringLibrary.Concat_StrStr` `Var Name` " " (`KismetStringLibrary.Conv_DoubleToString` Value)) null)))

(fn `SetCVars`
  (`self.SetCVar` "r.Mooa.DiffuseColorRamp.UVOffsetMaxRange" (`self.Diffuse Ramp Offset Max Range`))
  (`self.SetCVar` "r.Mooa.SpecularColorRamp.UVOffsetMaxRange" (`self.Specular Ramp Offset Max Range`))
  (`self.SetCVar` "r.Mooa.RimLight.MaxWidth" (`self.Rimlight Max Width`))
  (`self.SetCVar` "r.Mooa.RimLight.DepthTestThreshold" (`self.Rimlight Depth Test Threshold`))
  (`self.SetCVar` "r.Mooa.RimLight.DepthTestFadeDistance" (`self.Rimlight Depth Test Fade Distance`))
  (`self.SetCVar` "r.Mooa.HairShadow.Intensity" (`self.Hair Shadow Intensity`))
  (`self.SetCVar` "r.Mooa.HairShadow.Width" (`self.Hair Shadow Width`))
  (`self.SetCVar` "r.Mooa.HairShadow.DepthTestThreshold" (`self.Hair Shadow Depth Test Threshold`))
  (`self.SetCVar` "r.Mooa.HairShadow.DepthTestFadeDistance" (`self.Hair Shadow Depth Test Fade Distance`)))

(fn `SetPP`
  (bind _returnvalue (`self.GetPostComponent`))
  (setmembers `PostProcessSettings` :`StructRef` (`PostProcessComponent.Settings` _returnvalue) :`MooaExposureScale` (`self.Mooa Exposure Scale`) :`MooaLightSaturationScale` (`self.Light Saturation Scale`) :`MooaShadowColorIntensityDirectionalLights` (`self.Shadow Color Intensity Directional Lights`) :`MooaShadowColorIntensityPointLights` (`self.Shadow Color Intensity Point Lights`) :`MooaShadowColorIntensitySpotLights` (`self.Shadow Color Intensity Spot Lights`) :`MooaShadowColorIntensityRectLights` (`self.Shadow Color Intensity Rect Lights`) :`MooaGlobalIlluminationDirectionality` (`self.GI Directionality`) :`MooaGlobalIlluminationColor` (`self.GI Color`) :`MooaGlobalIlluminationIntensity` (`self.GI Intensity`) :`MooaShadowBias` (`self.Shadow Bias`) :`MooaRimLightIntensity` (`self.Rimlight Intensity`) :`MooaRimLightSaturationScale` (`self.Rimlight Saturation Scale`)))

(fn `UserConstructionScript`
  (`self.SetCVars`)
  (`self.SetPP`))